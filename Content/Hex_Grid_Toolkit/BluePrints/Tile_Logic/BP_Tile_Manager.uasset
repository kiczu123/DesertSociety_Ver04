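; Hex grid toolkit manager that spawns a MapSize-based map of BP_Tile actors into an axial-keyed TileMap, with a construction-script grid preview.
; It handles click and quit input directly and provides tile lookup by coordinate or type.
; Switched-off demos cover flood fill, Dijkstra flow maps, A* and beta FOV.
; Tick is empty, leaving mouse-hover tracing and debug drawing unwired, and an unexecuted graph serves as a toolkit glossary.
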(event `Key|Escape`
  (params (Key :type "Key Structure"))
  (:`Released`
    (`KismetSystemLibrary.QuitGame` null "Quit")))

(event `self.ReceiveBeginPlay`
  (bind _mapsize (`self.MapSize`))
  (bind _returnvalue (/ (* _mapsize -1) 2))
  (`InstancedStaticMeshComponent.ClearInstances` (`self.InstancedStaticMesh`))
  (`|ExecutionSequence`
    (:`then_0`
      ;[1 1 1] We are going to handle Input from this BP for simplicity but we should do it from Player Controller.
      (bind _output_get (set `self.PC_Ref` (`GameplayStatics.GetPlayerController` 0)))
      (set `PlayerController.bShowMouseCursor` true _output_get)
      (`self.EnableInput` _output_get))
    (:`then_1`
      (if true
        (bind _shapeout (`/Game/Hex_Grid_Toolkit/BluePrints/Hex_Logic/BPFL_Hex_Logic.getShape` "NewEnumerator1" (make `IntPoint` _returnvalue _returnvalue) (make `IntPoint` _mapsize _mapsize)))
        (for _array_element _shapeout
          (`self.spawnTile` _array_element))))))

(event `Key|Z` :consume false
  (params (Key :type "Key Structure")))

(event `UpdatePassable`
  (bind _tilemap (`self.TileMap`))
  (bind _shape (`self.findTilesOfType` _tilemap))
  (bind _output_get (set `self.Passable` _shape))
  (bind _shape_2 (`self.findTilesOfType` _tilemap "NewEnumerator9"))
  (`KismetArrayLibrary.Array_Append` _output_get _shape_2))

(event `HexSelectedUpdate`
  (bind _shape (`self.findTilesOfType` (`self.TileMap`) (`self.getTileType` (`self.HexSelected`))))
  (`|ExecutionSequence`
    (:`then_0`
      (if false
        (bind _shape_2 (`/Game/Hex_Grid_Toolkit/BluePrints/Hex_Logic/BPFL_Hex_Logic.FloodFill` _shape (`self.HexHover`)))
        (set `self.DisplayShape` _shape_2)))
    (:`then_1`
      (if false
        (bind _flowmap (`/Game/Hex_Grid_Toolkit/BluePrints/Hex_Logic/BPFL_Hex_Logic.Dijkstra` _shape (`self.HexSelected`)))
        (`/Game/Hex_Grid_Toolkit/BluePrints/Hex_Logic/BPFL_Hex_Logic.DebugDrawFlowMap` _flowmap 2.0)))))

(event `Key|LeftMouseButton` :consume false
  (params (Key :type "Key Structure"))
  (:`Pressed`
    ;[0 1 0] HexSelected
    (set `self.HexSelected` (`self.HexHover`))
    (`self.HexSelectedUpdate`)))

(event `self.ReceiveTick`
  (params (DeltaSeconds :type "Float (single-precision)")))

(event `HexHoverUpdate`
  (`|ExecutionSequence`
    (:`then_0`
      (if false
        (bind _path (`/Game/Hex_Grid_Toolkit/BluePrints/Hex_Logic/BPFL_Hex_Logic.PathFromFlowMap` (stale `HexSelectedUpdate` _flowmap) (`self.HexHover`)))
        (set `self.DisplayPath` _path)))
    (:`then_1`
      (if false
        (bind _path_2 (`/Game/Hex_Grid_Toolkit/BluePrints/Hex_Logic/BPFL_Hex_Logic.AStar` (stale `HexSelectedUpdate` _shape) (`self.HexSelected`) (`self.HexHover`)))
        (set `self.DisplayPath` _path_2)))
    (:`then_2`
      (if false
        (`self.setTileSight` (stale _onsight))
        (bind _shape (`self.findTilesOfType` (`self.TileMap`)))
        (bind _onsight (`/Game/Hex_Grid_Toolkit/BluePrints/Hex_Logic/BPFL_Hex_Logic.scanFov` (make `/Game/Hex_Grid_Toolkit/BluePrints/Hex_Logic/S_Scan_Fov` (`self.HexHover`) 12 0 _shape 0.0 6.0))) ; BETA STAGE
        (`self.setTileSight` _onsight true)))))

(fn `findTilesOfType`
  (params (TileMap :type "Map of IntPoint Structure to /Game/Hex_Grid_Toolkit/BluePrints/Tile_Logic/BP_Tile Object Reference (by ref)") (Type :type "/Game/Hex_Grid_Toolkit/BluePrints/Tile_Logic/E_TileType Enum" :default "NewEnumerator0"))
  (returns (Shape :type "Array of IntPoint Structure"))
  (locals (ShapeLocal :type "Array of IntPoint Structure"))
  (bind _keys (`BlueprintMapLibrary.Map_Keys` TileMap))
  (for _array_element _keys
    (if (`|EnumEquality` (`/Game/Hex_Grid_Toolkit/BluePrints/Tile_Logic/BP_Tile.Type` (`BlueprintMapLibrary.Map_Find` TileMap _array_element)) Type)
      (`KismetArrayLibrary.Array_Add` (`local.ShapeLocal`) _array_element)))
  (return (`local.ShapeLocal`)))

(fn `getTile`
  (params (Axial :type "IntPoint Structure (by ref)"))
  (returns (Tile :type "/Game/Hex_Grid_Toolkit/BluePrints/Tile_Logic/BP_Tile Object Reference"))
  (bind _value (`BlueprintMapLibrary.Map_Find` (`self.TileMap`) Axial))
  (`/Engine/EditorBlueprintResources/StandardMacros.IsValid` _value
    (:`Is Valid`
      (return _value))))

(fn `getTileType`
  (params (Axial :type "IntPoint Structure (by ref)"))
  (returns (Type :type "/Game/Hex_Grid_Toolkit/BluePrints/Tile_Logic/E_TileType Enum"))
  (bind _value (`BlueprintMapLibrary.Map_Find` (`self.TileMap`) Axial))
  (`/Engine/EditorBlueprintResources/StandardMacros.IsValid` _value
    (:`Is Valid`
      (return (`/Game/Hex_Grid_Toolkit/BluePrints/Tile_Logic/BP_Tile.Type` _value)))))

(fn `Hex_Logic_Definitions`
  (locals (Cube :type "IntVector Structure") (Axial :type "IntPoint Structure") (Offset :type "IntPoint Structure") (Polar :type "IntPoint Structure") (Location :type "Vector Structure") (Index :type Integer) (Steps :type Integer) (Degrees :type "Float (double-precision)") (Adjacent :type "/Game/Hex_Grid_Toolkit/BluePrints/Hex_Logic/E_Hex_Dir_Adjacent Enum") (Diagonal :type "/Game/Hex_Grid_Toolkit/BluePrints/Hex_Logic/E_Hex_Dir_Diagonal Enum") (Combined :type "/Game/Hex_Grid_Toolkit/BluePrints/Hex_Logic/E_Hex_Dir_Combined Enum") (Shape :type "Array of IntPoint Structure") (Path :type "Array of IntPoint Structure") (TileActorMap :type "Map of IntPoint Structure to /Game/Hex_Grid_Toolkit/BluePrints/Tile_Logic/BP_Tile Object Reference") (FlowMap :type "Map of IntPoint Structure to IntPoint Structure") (CostMap :type "Map of IntPoint Structure to Integer") (BP_Tile :type "/Game/Hex_Grid_Toolkit/BluePrints/Tile_Logic/BP_Tile Object Reference"))
  ;[1 0.6667 0] Dictionary of key concepts and naming conventions . To understand this toolkit.
)

(fn `setTileSight`
  (params (Axial :type "Array of IntPoint Structure") (bSight :type Boolean))
  (for _array_element Axial
    (bind (_value _returnvalue) (`BlueprintMapLibrary.Map_Find` (`self.TileMap`) _array_element))
    (if _returnvalue
      (`/Game/Hex_Grid_Toolkit/BluePrints/Tile_Logic/BP_Tile.FovSet` _value bSight))))

(fn `spawnTile`
  (params (Axial :type "IntPoint Structure") (Type :type "/Game/Hex_Grid_Toolkit/BluePrints/Tile_Logic/E_TileType Enum" :default "NewEnumerator0"))
  (bind (_value _returnvalue) (`BlueprintMapLibrary.Map_Find` (`self.TileMap`) Axial))
  (`|ExecutionSequence`
    (:`then_0`
      ;[1 1 1] If actor exist at that axial, destroy it
      (if _returnvalue
        (`self.K2_DestroyActor` _value)))
    (:`then_1`
      (bind _returnvalue_2 (`|SpawnActorFromClass` "/Game/Hex_Grid_Toolkit/BluePrints/Tile_Logic/BP_Tile.BP_Tile_C" (`KismetMathLibrary.MakeTransform` (0.0 0.0 0.0)) "Undefined" "OverrideRootScale" null Axial Type null))
      (`BlueprintMapLibrary.Map_Add` (`self.TileMap`) Axial _returnvalue_2))))

(fn `UserConstructionScript`
  (bind _instancedstaticmesh (`self.InstancedStaticMesh`))
  (bind _mapsize (`self.MapSize`))
  (bind _returnvalue (/ (* _mapsize -1) 2))
  (if (`self.ShowGrid`)
    (`InstancedStaticMeshComponent.ClearInstances` _instancedstaticmesh)
    (bind _shapeout (`/Game/Hex_Grid_Toolkit/BluePrints/Hex_Logic/BPFL_Hex_Logic.getShape` "NewEnumerator1" (make `IntPoint` _returnvalue _returnvalue) (make `IntPoint` _mapsize _mapsize)))
    (for _array_element _shapeout
      (bind (_location2d _location3d) (`/Game/Hex_Grid_Toolkit/BluePrints/Hex_Logic/BPFL_Hex_Logic.AxialToLocation` _array_element))
      (`InstancedStaticMeshComponent.AddInstance` _instancedstaticmesh (`KismetMathLibrary.MakeTransform` _location3d (`KismetMathLibrary.MakeRotator` 0.0)) false))))